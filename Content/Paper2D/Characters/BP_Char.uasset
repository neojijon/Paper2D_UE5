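; Paper2D side-scroller player character that runs along the X axis and attacks, using Enhanced Input.
; Tick flips control yaw by velocity direction, picks idle or run flipbooks, and plays footstep sounds on specific run frames.
; Attack plays a non-looping flipbook that blocks animation updates until finished.
; Its hit frames destroy actors overlapping the Box, activate Niagara and spawn BP_Bullet at a sprite socket, with DoOnce preventing repeat spawns.
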(event OnFinishedPlaying(Sprite)
  (bind _sprite (Variables|Default|GetSprite))
  ;[1 1 1] Attack
  (Variables|Default|SetisAttacking false)
  (Components|Timeline|SetLooping _sprite true)
  (Audio|Components|Audio|Play _sprite))

(event Custom|SetCharRotation
  ;[1 1 1] Char Rotation
  (Math|Float|CompareFloat (.x (Variables|/Script/Engine.MovementComponent|GetVelocity (Variables|Character|GetCharacterMovement))) 0.0
    (:>
      ;;[0 0.4745 1] Look Right
      (bind _asplayer_controller (Utilities|Casting|CastToPlayerController (Pawn|GetController)))
      (Pawn|SetControlRotation _asplayer_controller (Math|Rotator|MakeRotator 0.0 0.0 0.0)))
    (:<
      ;;[0 0.4745 1] Look Left
      (bind _asplayer_controller_2 (Utilities|Casting|CastToPlayerController (Pawn|GetController)))
      (Pawn|SetControlRotation _asplayer_controller_2 (Math|Rotator|MakeRotator 0.0 0.0 1.8e+02)))))

(event Custom|FootstepSound
  (bind _sprite (Variables|Default|GetSprite))
  (bind _returnvalue (Class|PaperFlipbookComponent|GetPlaybackPositioninFrames _sprite))
  ;[1 1 1] Foot Step Sound
  (if (== (Class|PaperFlipbookComponent|GetFlipbook (Variables|Default|GetSprite)) "/Game/Paper2D/Character/Animation/FB_Char_Run.FB_Char_Run")
    ;;[1 1 1] 1 or 5 에 발이 땅에 닿이면 소리가 나게 처리
    (if (or (== _returnvalue 1) (== _returnvalue 5))
      (Utilities|FlowControl|DoOnce false :!label _label
        (:Completed
          (Audio|PlaySoundatLocation "/Game/Maps/Assets/Bolt_2D_DinoRun_VE1/Audio/Land.Land" (Transformation|GetActorLocation) "0, 0, 0" 1.0 1.0 0.0 0 0 0 0)))
      (else
        (goto _label Reset)))))

(event Custom|CheckHitbox
  (bind _sprite (Variables|Default|GetSprite))
  (bind _returnvalue (Class|PaperFlipbookComponent|GetPlaybackPositioninFrames _sprite))
  (if (Variables|Default|GetisAttacking)
    (if (== (Class|PaperFlipbookComponent|GetFlipbook (Variables|Default|GetSprite)) "/Game/Paper2D/Character/Animation/FB_Char_Attack01.FB_Char_Attack01")
      (if (or (== _returnvalue 3) (== _returnvalue 6))
        (Utilities|FlowControl|Sequence
          (:then_0
            (for _array_element (Collision|GetOverlappingActors (Variables|Collision|GetBox) "/Script/Engine.Actor" :!class /Script/Engine.PrimitiveComponent)
              (if (!= _array_element self)
                (Actor|DestroyActor _array_element))))
          (:then_1
            (Utilities|FlowControl|DoOnce false :!label _label
              (:Completed
                (Components|Activation|Activate (Variables|Default|GetNiagara) true)
                (Game|SpawnActorfromClass "/Game/Paper2D/BP_Bullet.BP_Bullet_C" (Transformation|GetSocketTransform (Variables|Default|GetSprite) "ParticlePos" "RTS_World") "AlwaysSpawn" "MultiplyWithRoot" 0 0)))))
        (else
          (goto _label Reset))))))

(event Input|EnhancedActionEvents|EnhancedInputActionIA_Move
  (params (ActionValue :type Float%20%28double-precision%29) (ElapsedSeconds :type Float%20%28double-precision%29) (TriggeredSeconds :type Float%20%28double-precision%29) (InputAction :type Input%20Action%20Object%20Reference :default "/Game/Paper2D/Input/Actions/IA_Move.IA_Move"))
  ;[1 1 1] 키 메핑에 맞게  이동
  (Pawn|Input|AddMovementInput "1.000000,0.000000,0.000000" ActionValue false))

(event Input|EnhancedActionEvents|EnhancedInputActionIA_Attack
  (params (ActionValue :type Boolean) (ElapsedSeconds :type Float%20%28double-precision%29) (TriggeredSeconds :type Float%20%28double-precision%29) (InputAction :type Input%20Action%20Object%20Reference :default "/Game/Paper2D/Input/Actions/IA_Attack.IA_Attack"))
  (bind _sprite (Variables|Default|GetSprite))
  ;[1 1 1] Attack
  (Variables|Default|SetisAttacking true)
  (Components|Timeline|SetLooping _sprite false)
  (Sprite|SetFlipbook _sprite "/Game/Paper2D/Character/Animation/FB_Char_Attack01.FB_Char_Attack01"))

(event EventBeginPlay
  ;[1 1 1] 케릭터 키매핑
  (bind _asplayer_controller (Utilities|Casting|CastToPlayerController (Pawn|GetController)))
  (Input|AddMappingContext (PlayerController|LocalPlayerSubsystems|GetEnhancedInputLocalPlayerSubsystem _asplayer_controller) "/Game/Paper2D/Input/IMC_SideScroller.IMC_SideScroller" 0 "(bIgnoreAllPressedKeysUntilRelease=True,bForceImmediately=False,bNotifyUserSettings=False)"))

(event EventTick
  (params (DeltaSeconds :type Float%20%28single-precision%29))
  ;[1 1 1] Update
  (CallFunction|SetCharRotation)
  (CallFunction|UpdateAnimation)
  (CallFunction|FootstepSound)
  (CallFunction|CheckHitbox))

(fn ConstructionScript)

(fn UpdateAnimation
  ;[1 1 1] 코멘트
  (if (not (Variables|Default|GetisAttacking))
    (if (<= (Math|Float|Absolute(Float) (Math|Vector|VectorLength (Transformation|GetVelocity))) 0.0)
      (Sprite|SetFlipbook (Variables|Default|GetSprite) "/Game/Paper2D/Character/Animation/FB_Char_Idle.FB_Char_Idle")
      (else
        (Sprite|SetFlipbook (Variables|Default|GetSprite) "/Game/Paper2D/Character/Animation/FB_Char_Run.FB_Char_Run")))))